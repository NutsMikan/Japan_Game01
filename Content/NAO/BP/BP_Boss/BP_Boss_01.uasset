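; BP_Boss_01 is a boss actor with an HP value that drops when it takes damage.
; It enables player input on BeginPlay so a debug X key can apply fixed damage to the first BP_Boss_01 found in the level.
; AnyDamage subtracts the damage from HP and prints a message, with no death or zero-HP handling.
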(event `Key|X`
  (params (Key :type "Key Structure"))
  (:`Pressed`
    (`KismetSystemLibrary.PrintString` "x")
    (bind _outactors (`GameplayStatics.GetAllActorsOfClass` "BP_Boss_01_C"))
    (`GameplayStatics.ApplyDamage` (`|GetArrayItem` _outactors) 10.0)))

(event `self.ReceiveTick`
  (params (DeltaSeconds :type "Float (single-precision)")))

(event `self.ReceiveAnyDamage`
  (params (Damage :type "Float (single-precision)") (DamageType :type "DamageType Object Reference") (InstigatedBy :type "Controller Object Reference") (DamageCauser :type "Actor Object Reference"))
  (set `self.HP` (- (`self.HP`) Damage))
  (`KismetSystemLibrary.PrintString` "Damege"))

(event `self.ReceiveBeginPlay`
  ;[1 1 1] インプットキーを有効化
  (`self.EnableInput` (`GameplayStatics.GetPlayerController` 0)))

(fn `UserConstructionScript`)