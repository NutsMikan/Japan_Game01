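; BP_Bullet_2 is a gravity-free projectile that stops on hit and takes player key input directly.
; Debug-style keys stop it (L release), stop and delay-destroy it (T), or destroy it (Y).
; Key 3 runs a timeline lerping this actor from the first bullet toward the first SideScrollerCharacter, then destroys it, though comments describe pulling the character.
; Key 2 uses a looping timer to distinguish short and long presses, which only print.
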(event `Key|Y`
  (params (Key :type "Key Structure"))
  ;[1 1 1] Yキーで弾消去
  (:`Pressed`
    (`KismetSystemLibrary.PrintString` "delete")
    (`self.K2_DestroyActor`)))

(event `self.Box.OnComponentHit`
  (params (HitComponent :type "PrimitiveComponent Object Reference") (OtherActor :type "Actor Object Reference") (OtherComp :type "PrimitiveComponent Object Reference") (NormalImpulse :type "Vector Structure") (Hit :type "HitResult Structure (by ref)"))
  ;[1 1 1] 物に当たると止まって（　）秒後に消える
  (`KismetSystemLibrary.PrintString` "Hit")
  (`MovementComponent.StopMovementImmediately` (`self.ProjectileMovement`)))

(event `self.ReceiveBeginPlay`
  ;[1 1 1] インプットキーを有効化
  (`PrimitiveComponent.SetEnableGravity` (`self.Box`) false)
  (`self.EnableInput` (`GameplayStatics.GetPlayerController` 0)))

(event `Key|T`
  (params (Key :type "Key Structure"))
  ;[1 1 1] 重力
  (:`Pressed`
    (`KismetSystemLibrary.PrintString` "Push_T")
    (`MovementComponent.StopMovementImmediately` (`self.ProjectileMovement`))
    (`PrimitiveComponent.SetEnableGravity` (`self.Box`) false)
    (`KismetSystemLibrary.Delay` 0.8)
    (`self.K2_DestroyActor`)))

(event `Key|L`
  (params (Key :type "Key Structure"))
  ;[1 1 1] Lを離すと弾が消える
  (:`Released`
    (`MovementComponent.StopMovementImmediately` (`self.ProjectileMovement`))))

(event `self.ReceiveTick`
  (params (DeltaSeconds :type "Float (single-precision)")))

(event `Key|Three`
  (params (Key :type "Key Structure"))
  ;[1 1 1] 弾にキャラが引き寄せられる
  (:`Pressed`
    (`KismetSystemLibrary.PrintString` "hikiyose_02")
    ;;[1 1 1] キャラの座標を取得
    (bind _outactors (`GameplayStatics.GetAllActorsOfClass` "/Game/SideScrollerBP/Blueprints/SideScrollerCharacter.SideScrollerCharacter_C"))
    (set `self.Kyara` (`|GetArrayItem` _outactors))
    (bind _outactors_2 (`GameplayStatics.GetAllActorsOfClass` "BP_Bullet_2_C"))
    (set `self.Bullet02` (`|GetArrayItem` _outactors_2))
    (bind (_direction `_新規track_1`) (`Timeline|タイムライン_0` :!via `PlayFromStart`)
      (:`Update`
        (`self.K2_SetActorLocation` (`KismetMathLibrary.VLerp` (`self.K2_GetActorLocation` (`self.Bullet02`)) (`self.K2_GetActorLocation` (`self.Kyara`)) `_新規track_1`) true)
        (`KismetSystemLibrary.Delay` 1.0)
        (`self.K2_DestroyActor`) ; 消滅
      ))))

(event `Key|Two`
  (params (Key :type "Key Structure"))
  (:`Pressed`
    ;[1 1 1] キーを押した時刻を取得
    (set `self.StartTime` (`KismetMathLibrary.Now`))
    (bind _returnvalue (`KismetSystemLibrary.K2_SetTimerDelegate` (delegate `On Long Presu`) 0.1 true))
    (set `self.PressTimer` _returnvalue))
  (:`Released`
    ;[1 1 1] 短押し時の処理
    (`KismetSystemLibrary.K2_ClearAndInvalidateTimerHandle` (`self.PressTimer`)) ; 上のタイマーのループをクリア
    (if (< (`self.Press Time`) (`self.Long Press`))
      (`KismetSystemLibrary.PrintString` "Short") ; 短く推した時の処理
    )))

(event `On Long Presu`
  ;[1 1 1] 長押しの処理
  (bind _output_get (set `self.Press Time` (`KismetMathLibrary.GetTotalSeconds` (- (`KismetMathLibrary.Now`) (`self.StartTime`))))) ; 最初の値は0.1
  (if (>= _output_get (`self.Long Press`))
    (`KismetSystemLibrary.K2_ClearAndInvalidateTimerHandle` (`self.PressTimer`)) ; 上のタイマーのループをクリア
    (`KismetSystemLibrary.PrintString` "Long") ; 長押し時の処理
  ))

(fn `UserConstructionScript`)