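; BP_Douro_02_DM is a destructible mesh actor that fractures when struck by an actor tagged "Daruma".
; Its Destructible component's hit event applies radius damage at the impact point, with an impulse that scatters the fragments.
; BeginPlay enables player input for a Q key that only prints a debug message.
; ResetLocation is empty, and a delayed self-destroy chain is left unconnected.
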(event `self.Destructible.OnComponentHit`
  (params (HitComponent :type "PrimitiveComponent Object Reference") (OtherActor :type "Actor Object Reference") (OtherComp :type "PrimitiveComponent Object Reference") (NormalImpulse :type "Vector Structure") (Hit :type "HitResult Structure (by ref)"))
  (if (`self.ActorHasTag` OtherActor "Daruma")
    (`DestructibleComponent.ApplyRadiusDamage` (`self.Destructible`) 1.0 (`.ImpactPoint` (`GameplayStatics.BreakHitResult` Hit)) 100.0 2000.0 false) ; DamageRadius」の値が小さければ小さいほど、破壊される範囲が小さくなります。\n\nImpulseStrength」は値によって破片の飛び散り方が違います。\n値が小さいほど、破片は静かに、おとなしく落ちてゆく。\n\n値が大きいほど、破片は勢いよく飛んでいきます。\n\n\n「BaseDamage」は1以上なら問題ない気がします。（適当）
  ))

(event `Key|Q`
  (params (Key :type "Key Structure"))
  (:`Pressed`
    (`KismetSystemLibrary.PrintString` "Hello")))

(event `self.ReceiveBeginPlay`
  ;[1 1 1] インプットキーを有効化
  (`self.EnableInput` (`GameplayStatics.GetPlayerController` 0)))

(fn `UserConstructionScript`)